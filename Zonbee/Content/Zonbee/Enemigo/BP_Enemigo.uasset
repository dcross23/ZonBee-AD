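; BP_Enemigo is the round-based zombie enemy, which registers itself in ThirdPersonGameMode's enemy count on spawn.
; It wanders randomly on delayed Ticks until PawnSensing spots the player, then runs over and opens a timed attack window in which ColisionGolpe damages once.
; BP_Bala overlaps show a hitmarker, subtract health and draw it toward the player.
; Death decrements the count, triggers last-enemy effects at zero and randomly drops ammo, sometimes with a shield.
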(event `self.ReceiveBeginPlay`
  ;[1 1 1] Cuando se cree el enemigo, aumenta en 1 los enemigos de la ronda
  (bind _asthird_person_game_mode (cast `/Game/Zonbee/OtrosBlueprints/ThirdPersonGameMode` (`GameplayStatics.GetGameMode`)))
  (`/Engine/EditorBlueprintResources/StandardMacros.IncrementInt` (`/Game/Zonbee/OtrosBlueprints/ThirdPersonGameMode.EnemigosRonda` _asthird_person_game_mode)
    (:`  `
      (`GameplayStatics.PlaySoundAtLocation` "/Game/Zonbee/Sonidos/S_Zombie.S_Zombie" (`self.K2_GetActorLocation` self) (struct) 1.0 1.0 0.0 null null null))))

(event `self.ReceiveActorBeginOverlap`
  (params (OtherActor :type "Actor Object Reference"))
  (bind _returnvalue (`KismetMathLibrary.RandomIntegerInRange` 0 99))
  (bind _returnvalue_2 (`self.K2_GetActorLocation`))
  (bind _returnvalue_3 (`self.GetTransform`))
  ;[1 1 1] Evento para que el reciba daño y se gire a por el jugador cuando sea disparado
  (if (not (`self.Morir`))
    (bind _asbp_bala (cast `/Game/Zonbee/Objetos/Balas/BP_Bala` OtherActor))
    (bind _returnvalue_4 (`|CreateWidget` "/Game/Zonbee/Widgets/WP_Hitmarker.WP_Hitmarker_C"))
    (`UserWidget.AddToViewport` _returnvalue_4 0)
    (bind _output_get (set `self.VidaEnemigo` (- (`self.VidaEnemigo`) (`self.DañoPorBala`))))
    (if (<= _output_get 0)
      (`MovementComponent.StopMovementImmediately` (`self.CharacterMovement`))
      (set `self.Morir` true)
      (`PrimitiveComponent.SetCollisionEnabled` (`self.CapsuleComponent`) "NoCollision")
      (`GameplayStatics.SpawnEmitterAtLocation` "/Game/InfinityBladeEffects/Effects/FX_Mobile/Impacts/P_Impact_Player_Ice_Medium.P_Impact_Player_Ice_Medium" (`self.K2_GetActorLocation`))
      (bind _asthird_person_game_mode (cast `/Game/Zonbee/OtrosBlueprints/ThirdPersonGameMode` (`GameplayStatics.GetGameMode`)))
      (bind _result (`/Engine/EditorBlueprintResources/StandardMacros.DecrementInt` (`/Game/Zonbee/OtrosBlueprints/ThirdPersonGameMode.EnemigosRonda` _asthird_person_game_mode))
        (:`  `
          (`/Game/Zonbee/OtrosBlueprints/ThirdPersonGameMode.ComprobarEnemigosRestantes` _asthird_person_game_mode)
          (if (== _result 0)
            (`GameplayStatics.SpawnEmitterAtLocation` "/Game/InfinityBladeEffects/Effects/FX_Monsters/FX_Monster_Ausar/P_AU_Trap_Impact.P_AU_Trap_Impact" _returnvalue_2)
            (`GameplayStatics.PlaySoundAtLocation` "/Game/Zonbee/Sonidos/S_ExplosionRonda.S_ExplosionRonda" _returnvalue_2 (struct) 1.0 1.0 0.0 null null null))
          (if (< _returnvalue 30)
            (`|SpawnActorFromClass` "/Game/Zonbee/Objetos/Municion/BP_CajaMunicion.BP_CajaMunicion_C" _returnvalue_3 "Undefined" "OverrideRootScale" null null)
            (if (and (< _returnvalue 50) (> _returnvalue 30))
              (`|SpawnActorFromClass` "/Game/Zonbee/Objetos/Escudo/BP_Escudo.BP_Escudo_C" _returnvalue_3 "Undefined" "OverrideRootScale" null null)))))
      (else
        (`GameplayStatics.SpawnEmitterAtLocation` "/Game/InfinityBladeEffects/Effects/FX_Mobile/Impacts/P_Impact_Shield_Fire.P_Impact_Shield_Fire" (`self.K2_GetActorLocation` _asbp_bala))
        (`|AIMoveTo` self (0.0 0.0 0.0) (`GameplayStatics.GetPlayerCharacter` 0))))))

(event `self.PawnSensing.OnSeePawn`
  (params (Pawn :type "Pawn Object Reference"))
  ;[1 1 1] Evento para que el enemigo siga al jugador cuando lo vea
  (if (not (`self.Morir`))
    (set `self.SeguirJugador` true)
    (bind _asbp_jugador (cast `/Game/Zonbee/Jugador/BP_Jugador` Pawn))
    (set `CharacterMovementComponent.MaxWalkSpeed` (`self.VelocidadCorriendo`) (`self.CharacterMovement`))
    (`|AIMoveTo` self (0.0 0.0 0.0) _asbp_jugador
      (:`OnSuccess`
        (if (not (`self.Atacar`))
          (set `self.Atacar` true)
          (`GameplayStatics.PlaySoundAtLocation` "/Game/Zonbee/Sonidos/S_ZombieAtaque.S_ZombieAtaque" (`self.K2_GetActorLocation` self) (struct) 1.0 1.0 0.0 null null null)
          (`KismetSystemLibrary.Delay` 2.5)
          (set `self.Atacar` false)
          (set `self.HaAtacado` false)
          (set `self.SeguirJugador` false :!label _label)))
      (:`OnFail`
        (goto _label)))))

(event `self.ReceiveTick`
  (params (DeltaSeconds :type "Float (single-precision)"))
  ;[1 1 1] Si no está siguiendo al jugador, se va a mover aleatoriamente
  (`KismetSystemLibrary.Delay` (`KismetMathLibrary.RandomFloatInRange` 2.0 5.0))
  (if (`self.Morir`)
    _
    (elif (not (`self.SeguirJugador`))
      (set `CharacterMovementComponent.MaxWalkSpeed` (`self.VelocidadAndando`) (`self.CharacterMovement`))
      (`|AIMoveTo` self (`NavigationSystemV1.K2_GetRandomReachablePointInRadius` (`self.K2_GetActorLocation`) 400.0 null null) null))))

(event `self.ColisionGolpe.OnComponentBeginOverlap`
  (params (OverlappedComponent :type "PrimitiveComponent Object Reference") (OtherActor :type "Actor Object Reference") (OtherComp :type "PrimitiveComponent Object Reference") (OtherBodyIndex :type Integer) (bFromSweep :type Boolean) (SweepResult :type "HitResult Structure (by ref)"))
  ;[1 1 1] Atacar al jugador
  (bind _asbp_jugador (cast `/Game/Zonbee/Jugador/BP_Jugador` OtherActor))
  (if (and (`self.Atacar`) (not (`self.HaAtacado`)))
    (`/Game/Zonbee/Jugador/BP_Jugador.RecibirDaño` _asbp_jugador)
    (set `self.HaAtacado` true)))

(fn `UserConstructionScript`)