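; AK weapon actor that handles firing and magazine reloading.
; Disparar, while rounds remain, spawns a BP_Bala at the mesh's Muzzle socket with a shot sound, decrements Balas and spawns a muzzle flash.
; The flash takes its socket from player 0's equipped Arma via a BP_Jugador cast, not from its own mesh.
; RecargarBalas refills the magazine from BalasRestantes, using whatever remains when reserves fall short.
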(event `Disparar`
  (if (> (`self.Balas`) 0)
    (`self.Crear Bala`)
    (`/Engine/EditorBlueprintResources/StandardMacros.DecrementInt` (`self.Balas`)
      (:`  `
        (`self.CrearLuzDisparo`)))))

(fn `Crear Bala`
  (bind _skeletalmesh (`self.SkeletalMesh`))
  (`|SpawnActorFromClass` "/Game/Zonbee/Objetos/Balas/BP_Bala.BP_Bala_C" (`SceneComponent.GetSocketTransform` _skeletalmesh "Muzzle" "RTS_World") "Undefined" "OverrideRootScale" null null)
  (`GameplayStatics.PlaySoundAtLocation` "/Game/StarterContent/Audio/Explosion01.Explosion01" (`SceneComponent.GetSocketLocation` _skeletalmesh "None") (struct) 1.0 1.0 0.0 null null null))

(fn `CrearLuzDisparo`
  (bind _asbp_jugador (cast `/Game/Zonbee/Jugador/BP_Jugador` (`GameplayStatics.GetPlayerCharacter` 0)))
  (bind _skeletalmesh (`/Game/Zonbee/Arma/BP_AK_Actor.SkeletalMesh` (`/Game/Zonbee/Jugador/BP_Jugador.Arma` _asbp_jugador)))
  (`GameplayStatics.SpawnEmitterAtLocation` "/Game/InfinityBladeEffects/Effects/FX_Monsters/FX_Monster_Chicken/P_ChickenMaster_MuzzleFlash_01.P_ChickenMaster_MuzzleFlash_01" (`SceneComponent.GetSocketLocation` _skeletalmesh "Muzzle") (`SceneComponent.GetSocketRotation` _skeletalmesh "Muzzle") (0.05 0.05 0.05)))

(fn `RecargarBalas`
  (bind _output_get (set `self.BalasDisparadas` (- (`self.BalasTotalesCargador`) (`self.Balas`))))
  (if (> _output_get 0)
    (if (>= (`self.BalasRestantes`) (`self.BalasDisparadas`))
      (set `self.Balas` (`self.BalasTotalesCargador`))
      (set `self.BalasRestantes` (- (`self.BalasRestantes`) (`self.BalasDisparadas`)))
      (else
        (set `self.Balas` (+ (`self.BalasRestantes`) (`self.Balas`)))
        (set `self.BalasRestantes` 0)))))

(fn `UserConstructionScript`)