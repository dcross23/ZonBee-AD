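; BP_Escudo is a shield pickup that restores part of the player's Escudo (shield) value on touch.
; On overlap it casts the other actor to BP_Jugador, ignores anything else, and adds a fixed amount capped at the maximum.
; It then plays the item sound at its location and destroys itself, even if the shield was already full.
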(event `self.ReceiveActorBeginOverlap`
  (params (OtherActor :type "Actor Object Reference"))
  (bind _asbp_jugador (cast `/Game/Zonbee/Jugador/BP_Jugador` OtherActor))
  (bind _escudo (`/Game/Zonbee/Jugador/BP_Jugador.Escudo` _asbp_jugador))
  (if (< _escudo 100)
    (bind _returnvalue (+ _escudo 25))
    (if (> _returnvalue 100)
      (set `/Game/Zonbee/Jugador/BP_Jugador.Escudo` 100 _asbp_jugador)
      (else
        (set `/Game/Zonbee/Jugador/BP_Jugador.Escudo` _returnvalue _asbp_jugador))))
  (`GameplayStatics.PlaySoundAtLocation` "/Game/Zonbee/Sonidos/S_Item.S_Item" (`self.K2_GetActorLocation`) (struct) 1.0 1.0 0.0 null null null)
  (`self.K2_DestroyActor`))

(fn `UserConstructionScript`)