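; BP_CajaMunicion is an ammo box pickup that refills the player's weapon reserve on overlap.
; When a BP_Jugador overlaps it and the weapon's remaining bullets are below the maximum, it adds one magazine's worth, clamped to that maximum.
; It then plays the item sound at its location and destroys itself, even if the reserve was already full.
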(event `self.ReceiveActorBeginOverlap`
  (params (OtherActor :type "Actor Object Reference"))
  (bind _asbp_jugador (cast `/Game/Zonbee/Jugador/BP_Jugador` OtherActor))
  (bind _arma (`/Game/Zonbee/Jugador/BP_Jugador.Arma` _asbp_jugador))
  (bind _balasrestantes (`/Game/Zonbee/Arma/BP_AK_Actor.BalasRestantes` _arma))
  (if (< _balasrestantes (`/Game/Zonbee/Arma/BP_AK_Actor.BalasMaxRestantes` _arma))
    (bind _output_get (set `/Game/Zonbee/Arma/BP_AK_Actor.BalasRestantes` (+ _balasrestantes (`/Game/Zonbee/Arma/BP_AK_Actor.BalasTotalesCargador` _arma)) _arma))
    (bind _balasmaxrestantes (`/Game/Zonbee/Arma/BP_AK_Actor.BalasMaxRestantes` _arma))
    (if (> _output_get _balasmaxrestantes)
      (set `/Game/Zonbee/Arma/BP_AK_Actor.BalasRestantes` _balasmaxrestantes _arma)))
  (`GameplayStatics.PlaySoundAtLocation` "/Game/Zonbee/Sonidos/S_Item.S_Item" (`self.K2_GetActorLocation`) (struct) 1.0 1.0 0.0 null null null)
  (`self.K2_DestroyActor`))

(fn `UserConstructionScript`)