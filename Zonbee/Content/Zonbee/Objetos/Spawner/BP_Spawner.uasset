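; BP_Spawner is a wave spawner that creates BP_Enemigo enemies at the start of each round.
; On BeginPlay it binds its SiguienteRonda event to the next-round dispatcher on ThirdPersonGameMode.
; Each call spawns NumEnemigos enemies at random reachable navmesh points within a fixed radius of the spawner, then raises the count by two for the following round.
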(event `self.ReceiveBeginPlay`
  (bind _asthird_person_game_mode (cast `/Game/Zonbee/OtrosBlueprints/ThirdPersonGameMode` (`GameplayStatics.GetGameMode`)))
  (add `/Game/Zonbee/OtrosBlueprints/ThirdPersonGameMode.SiguienteRonda` _asthird_person_game_mode (delegate `SiguienteRonda`)))

(event `SiguienteRonda`
  (for _ (range 1 (+ (`self.NumEnemigos`) 1))
    (`|SpawnActorFromClass` "/Game/Zonbee/Enemigo/BP_Enemigo.BP_Enemigo_C" (`KismetMathLibrary.MakeTransform` (`NavigationSystemV1.K2_GetRandomReachablePointInRadius` (`self.K2_GetActorLocation`) 300.0 null null) (`self.K2_GetActorRotation`)) "Undefined" "OverrideRootScale" null null))
  (set `self.NumEnemigos` (+ 2 (`self.NumEnemigos`))))

(fn `UserConstructionScript`)